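; BP_DialogueBox is a trigger volume that starts and advances a range of dialogue lines while the first-person character stands inside.
; On overlap it flags the character, enables interact input, finds BP_DialogueManager and shows dialogue if the shared index matches its start index.
; Each interact increments the manager's index and shows the next line until the last index, where the ending event is an empty stub.
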(event `self.Box.OnComponentBeginOverlap`
  (params (OverlappedComponent :type "PrimitiveComponent Object Reference") (OtherActor :type "Actor Object Reference") (OtherComp :type "PrimitiveComponent Object Reference") (OtherBodyIndex :type Integer) (bFromSweep :type Boolean) (SweepResult :type "HitResult Structure (by ref)"))
  (bind _asbp_first_person_character (cast `/Game/FirstPerson/Blueprints/BP_FirstPersonCharacter` OtherActor))
  (set `/Game/FirstPerson/Blueprints/BP_FirstPersonCharacter.InDialogueBox?` true _asbp_first_person_character)
  (`self.EnableInput` (`GameplayStatics.GetPlayerController` 0))
  (bind _returnvalue (`GameplayStatics.GetActorOfClass` "/Game/_Romain/LevelElements/BP_DialogueManager.BP_DialogueManager_C"))
  (set `self.ManagerRef` _returnvalue)
  (if (== (`self.DialogueStartIndex`) (`/Game/_Romain/LevelElements/BP_DialogueManager.DialogueIndex` (`self.ManagerRef`)))
    (`self.OnVerifiedDialogueIndex`)
    (else
      (`KismetSystemLibrary.PrintString` "error:WrongDialogueIndex"))))

(event `self.Box.OnComponentEndOverlap`
  (params (OverlappedComponent :type "PrimitiveComponent Object Reference") (OtherActor :type "Actor Object Reference") (OtherComp :type "PrimitiveComponent Object Reference") (OtherBodyIndex :type Integer))
  (bind _asbp_first_person_character (cast `/Game/FirstPerson/Blueprints/BP_FirstPersonCharacter` OtherActor))
  (set `/Game/FirstPerson/Blueprints/BP_FirstPersonCharacter.InDialogueBox?` false _asbp_first_person_character)
  (`self.DisableInput` (`GameplayStatics.GetPlayerController` 0)))

(event `EnhancedInput|/Game/FirstPerson/Input/Actions/IA_Interact`
  (params (ActionValue :type Boolean) (ElapsedSeconds :type "Float (double-precision)") (TriggeredSeconds :type "Float (double-precision)") (InputAction :type "InputAction Object Reference" :default "/Game/FirstPerson/Input/Actions/IA_Interact.IA_Interact"))
  (:`Started`
    (`self.OnNextDialogue`)))

(event `OnVerifiedDialogueIndex`
  (`/Game/_Romain/LevelElements/BP_DialogueManager.OnSetDialogue` (`self.ManagerRef`)))

(event `OnNextDialogue`
  (bind _dialogueindex (`/Game/_Romain/LevelElements/BP_DialogueManager.DialogueIndex` (`self.ManagerRef`)))
  (bind _result (`/Engine/EditorBlueprintResources/StandardMacros.IncrementInt` _dialogueindex)
    (:`  `
      (`KismetSystemLibrary.PrintString` (`KismetStringLibrary.Conv_IntToString` _dialogueindex))
      (if (== _result (`self.DialogueLastIndex`))
        (`self.OnEndingDialogue`)
        (else
          (`self.OnVerifiedDialogueIndex`))))))

(event `OnEndingDialogue`)

(fn `UserConstructionScript`)