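; NPC dialogue trigger that lets the player talk to a character and, for Mickael, shoot them afterwards.
; Box overlap shows the interact prompt and enables input if the shared BP_DialogueManager index matches its start index.
; Interact starts and advances lines up to the last index, freezing player input until the end event fires.
; Once dialogue ends, a projectile hit hides Mickael and marks him dead on the end objective.
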(event `self.Box.OnComponentBeginOverlap`
  (params (OverlappedComponent :type "PrimitiveComponent Object Reference") (OtherActor :type "Actor Object Reference") (OtherComp :type "PrimitiveComponent Object Reference") (OtherBodyIndex :type Integer) (bFromSweep :type Boolean) (SweepResult :type "HitResult Structure (by ref)"))
  (bind _asbp_first_person_character (cast `/Game/FirstPerson/Blueprints/BP_FirstPersonCharacter` OtherActor))
  (set `/Game/FirstPerson/Blueprints/BP_FirstPersonCharacter.InDialogueBox?` true _asbp_first_person_character)
  (bind _returnvalue (`GameplayStatics.GetActorOfClass` "/Game/_Romain/LevelElements/BP_DialogueManager.BP_DialogueManager_C"))
  (set `self.ManagerRef` _returnvalue)
  (bind _returnvalue_2 (`GameplayStatics.GetActorOfClass` "/Game/_Romain/LevelElements/BP_UIManager.BP_UIManager_C"))
  (set `Widget.Visibility` "Visible" (`/Game/_Romain/UI/UI_MainWidget.UI_Interact` (`/Game/_Romain/LevelElements/BP_UIManager.WidgetRef` _returnvalue_2)))
  (if (== (`self.DialogueStartIndex`) (`/Game/_Romain/LevelElements/BP_DialogueManager.DialogueIndex` (`self.ManagerRef`)))
    (`self.EnableInput` (`GameplayStatics.GetPlayerController` 0))
    (else
      (`KismetSystemLibrary.PrintString` "error:WrongDialogueIndex"))))

(event `self.Box.OnComponentEndOverlap`
  (params (OverlappedComponent :type "PrimitiveComponent Object Reference") (OtherActor :type "Actor Object Reference") (OtherComp :type "PrimitiveComponent Object Reference") (OtherBodyIndex :type Integer))
  (bind _asbp_first_person_character (cast `/Game/FirstPerson/Blueprints/BP_FirstPersonCharacter` OtherActor))
  (set `/Game/FirstPerson/Blueprints/BP_FirstPersonCharacter.InDialogueBox?` false _asbp_first_person_character)
  (`self.DisableInput` (`GameplayStatics.GetPlayerController` 0))
  (bind _returnvalue (`GameplayStatics.GetActorOfClass` "/Game/_Romain/LevelElements/BP_UIManager.BP_UIManager_C"))
  (set `Widget.Visibility` "Hidden" (`/Game/_Romain/UI/UI_MainWidget.UI_Interact` (`/Game/_Romain/LevelElements/BP_UIManager.WidgetRef` _returnvalue))))

(event `StartDialogue`
  (`/Game/_Romain/LevelElements/BP_DialogueManager.OnShowDialogue` (`self.ManagerRef`))
  (`self.OnVerifiedDialogueIndex`)
  (`self.DisableInput` (`GameplayStatics.GetPlayerCharacter` 0) (`GameplayStatics.GetPlayerController` 0))
  (set `self.IsDialogueRunning?` true))

(event `OnVerifiedDialogueIndex`
  (`/Game/_Romain/LevelElements/BP_DialogueManager.OnSetDialogue` (`self.ManagerRef`)))

(event `EnhancedInput|/Game/FirstPerson/Input/Actions/IA_Interact`
  (params (ActionValue :type Boolean) (ElapsedSeconds :type "Float (double-precision)") (TriggeredSeconds :type "Float (double-precision)") (InputAction :type "InputAction Object Reference" :default "/Game/FirstPerson/Input/Actions/IA_Interact.IA_Interact"))
  (:`Started`
    (if (== (`self.DialogueStartIndex`) (`/Game/_Romain/LevelElements/BP_DialogueManager.DialogueIndex` (`self.ManagerRef`)))
      (if (`self.IsDialogueRunning?`)
        (if (< (`/Game/_Romain/LevelElements/BP_DialogueManager.DialogueIndex` (`self.ManagerRef`)) (`self.DialogueLastIndex`)) :!label _label
          (`self.OnNextDialogue`))
        (else
          (`self.StartDialogue`)))
      (else
        (goto _label)))))

(event `OnNextDialogue`
  (bind _result (`/Engine/EditorBlueprintResources/StandardMacros.IncrementInt` (`/Game/_Romain/LevelElements/BP_DialogueManager.DialogueIndex` (`self.ManagerRef`)))
    (:`  `
      (if (== _result (`self.DialogueLastIndex`))
        (`self.OnEndingDialogue`)
        (else
          (`self.OnVerifiedDialogueIndex`))))))

(event `OnEndingDialogue`
  (`self.EnableInput` (`GameplayStatics.GetPlayerCharacter` 0) (`GameplayStatics.GetPlayerController` 0))
  (`/Game/_Romain/LevelElements/BP_DialogueManager.OnHideDialogue` (`self.ManagerRef`))
  (bind _returnvalue (`GameplayStatics.GetActorOfClass` "/Game/_Romain/LevelElements/BP_NarrativeManager.BP_NarrativeManager_C"))
  (`self.OnDialogueEnd`)
  (set `self.canBeKilled` true))

(event `SetRenata`
  (`SkeletalMeshComponent.SetSkeletalMeshAsset` (`self.SkeletalMesh`) "/Game/Characters/Mannequins/Meshes/SKM_Quinn.SKM_Quinn"))

(event `self.Capsule.OnComponentBeginOverlap`
  (params (OverlappedComponent :type "PrimitiveComponent Object Reference") (OtherActor :type "Actor Object Reference") (OtherComp :type "PrimitiveComponent Object Reference") (OtherBodyIndex :type Integer) (bFromSweep :type Boolean) (SweepResult :type "HitResult Structure (by ref)"))
  (bind _asbp_first_person_projectile (cast `/Game/FirstPerson/Blueprints/BP_FirstPersonProjectile` OtherActor))
  (`self.K2_DestroyActor` _asbp_first_person_projectile)
  (if (`self.canBeKilled`)
    (if (`self.isMickael`)
      (`self.OnKilled`)
      (`SceneComponent.SetVisibility` (`self.SkeletalMesh`) false false))))

(event `OnKilled`
  (bind _returnvalue (`GameplayStatics.GetActorOfClass` "/Game/_Corentin/Blueprint/BP_Objective_Interact_END.BP_Objective_Interact_END_C"))
  (set `/Game/_Corentin/Blueprint/BP_Objective_Interact_END.isMickaelDead` true _returnvalue)
  (`/Game/_Corentin/Blueprint/BP_Objective_Interact_END.RefreshDescription` _returnvalue))

(fn `UserConstructionScript`)