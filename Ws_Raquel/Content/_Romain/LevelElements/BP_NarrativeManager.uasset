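; BP_NarrativeManager sequences narrative objectives, starting the first valid one when play begins.
; On BeginPlay it resets ObjectiveIndex on the first-person player character, then sets the current objective from the Objectives list.
; Each valid objective gets its end-condition event bound before being activated.
; OnNextObjective clears the current objective, increments the index and activates the following entry, forming an event-driven chain.
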(event `self.ReceiveBeginPlay`
  (bind _asbp_first_person_character (cast `/Game/FirstPerson/Blueprints/BP_FirstPersonCharacter` (`GameplayStatics.GetPlayerCharacter` 0)))
  (set `/Game/FirstPerson/Blueprints/BP_FirstPersonCharacter.objectiveIndex` 0 _asbp_first_person_character)
  (`self.OnSetObjective`))

(event `OnSetObjective`
  (bind _currentobjective (`self.currentObjective`))
  (set `self.currentObjective` (`|GetArrayItem` (`self.Objectives`) (`self.ObjectiveIndex`)))
  (`/Engine/EditorBlueprintResources/StandardMacros.IsValid` _currentobjective
    (:`Is Valid`
      (add `/Game/_Corentin/Blueprint/BP_Objective.OnEndCondition` _currentobjective (`|CreateDelegate` :!event `OnNextObjective`))
      (`/Game/_Corentin/Blueprint/BP_Objective.ActivateEvent` (`self.currentObjective`)))))

(event `OnNextObjective`
  (set `self.currentObjective` null)
  (`/Engine/EditorBlueprintResources/StandardMacros.IncrementInt` (`self.ObjectiveIndex`)
    (:`  `
      (`self.OnSetObjective`))))

(fn `UserConstructionScript`)