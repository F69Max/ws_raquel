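; A go-to objective actor that completes when the first-person player character enters its trigger box.
; It starts deactivated at BeginPlay; activation and deactivation events toggle an IsActive flag and the zone indicator's visibility.
; An overlap while active deactivates it, prints a completion message and calls OnEndCondition to signal the end.
; A delayed self-activation chain is left disconnected, so activation must come from outside this graph.
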(event `self.ReceiveTick`
  (params (DeltaSeconds :type "Float (single-precision)")))

(event `self.ReceiveBeginPlay`
  (`self.DesactivateEvent`))

(event `self.ActivateEvent`
  (set `self.isActive` true)
  (`SceneComponent.SetVisibility` (`self.ZoneIndicator`) true false)
  (`KismetSystemLibrary.PrintString` "Objective Init" true true (struct :`G` 0.66 :`B` 1.0 :`A` 1.0) 5.0))

(event `self.DesactivateEvent`
  (set `self.isActive` false)
  (`SceneComponent.SetVisibility` (`self.ZoneIndicator`) false false))

(event `self.Box.OnComponentBeginOverlap`
  (params (OverlappedComponent :type "PrimitiveComponent Object Reference") (OtherActor :type "Actor Object Reference") (OtherComp :type "PrimitiveComponent Object Reference") (OtherBodyIndex :type Integer) (bFromSweep :type Boolean) (SweepResult :type "HitResult Structure (by ref)"))
  (if (`self.isActive`)
    (cast `/Game/FirstPerson/Blueprints/BP_FirstPersonCharacter` OtherActor)
    (`self.DesactivateEvent`)
    (`KismetSystemLibrary.PrintString` "Objective Complete" true true (struct :`R` 1.0 :`B` 0.080226 :`A` 1.0) 5.0)
    (`self.OnEndCondition`)))

(fn `UserConstructionScript`
  (`parent.UserConstructionScript`))