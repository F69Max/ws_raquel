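; BP_Objective_Interact_END is the interactable quest objective that triggers the end condition, built around an act of execution.
; RefreshDescription sets the objective text from IsMickaelDead: submit the act if Mickael is dead, otherwise throw it in the fire.
; Interact deactivates the event, calls the end condition and prints a debug "END QUEST" message.
; BeginPlay and the construction script only defer to the parent class.
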(event `self.ReceiveBeginPlay`
  (`parent.ReceiveBeginPlay`))

(event `RefreshDescription`
  (if (`self.isMickaelDead`)
    (set `self.informations` (make `/Game/_Romain/Utilities/F_Objective` "" "Submit the act of execution"))
    (else
      (set `self.informations` (make `/Game/_Romain/Utilities/F_Objective` "" "Throw the act of execution in the fire")))))

(event `self.Interact`
  (`self.DesactivateEvent`)
  (`self.OnEndCondition`)
  (`KismetSystemLibrary.PrintString` "END QUEST"))

(fn `UserConstructionScript`
  (`parent.UserConstructionScript`))