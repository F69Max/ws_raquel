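; BP_Objective_Interact is an objective that the first-person character completes by interacting with it.
; It starts deactivated, and its activate and deactivate events toggle the Interactable component's visibility and collision.
; While active, overlapping InteractRange registers it as the character's current interaction objective, cleared on exit.
; Interact deactivates it and calls the end condition, with debug prints on activation and completion.
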(event `self.ReceiveBeginPlay`
  (`self.DesactivateEvent`))

(event `self.ActivateEvent`
  (bind _interactable (`self.Interactable`))
  (bind _informations_objectivename (break `/Game/_Romain/Utilities/F_Objective` (`self.informations`)))
  (set `self.isActive` true)
  (`SceneComponent.SetVisibility` _interactable true false)
  (`PrimitiveComponent.SetCollisionEnabled` _interactable "QueryAndPhysics")
  (`KismetSystemLibrary.PrintString` "Event Activate")
  (`KismetSystemLibrary.PrintString` _informations_objectivename true true (struct :`G` 0.66 :`B` 1.0 :`A` 1.0) 5.0))

(event `self.DesactivateEvent`
  (bind _interactable (`self.Interactable`))
  (set `self.isActive` false)
  (`SceneComponent.SetVisibility` _interactable false false)
  (`PrimitiveComponent.SetCollisionEnabled` _interactable "NoCollision"))

(event `self.InteractRange.OnComponentBeginOverlap`
  (params (OverlappedComponent :type "PrimitiveComponent Object Reference") (OtherActor :type "Actor Object Reference") (OtherComp :type "PrimitiveComponent Object Reference") (OtherBodyIndex :type Integer) (bFromSweep :type Boolean) (SweepResult :type "HitResult Structure (by ref)"))
  (bind _asbp_first_person_character (cast `/Game/FirstPerson/Blueprints/BP_FirstPersonCharacter` OtherActor))
  (if (`self.isActive`)
    (set `/Game/FirstPerson/Blueprints/BP_FirstPersonCharacter.isInInteractionRange` true _asbp_first_person_character)
    (set `/Game/FirstPerson/Blueprints/BP_FirstPersonCharacter.actualInteractObjective` self _asbp_first_person_character)))

(event `self.InteractRange.OnComponentEndOverlap`
  (params (OverlappedComponent :type "PrimitiveComponent Object Reference") (OtherActor :type "Actor Object Reference") (OtherComp :type "PrimitiveComponent Object Reference") (OtherBodyIndex :type Integer))
  (bind _asbp_first_person_character (cast `/Game/FirstPerson/Blueprints/BP_FirstPersonCharacter` OtherActor))
  (set `/Game/FirstPerson/Blueprints/BP_FirstPersonCharacter.isInInteractionRange` false _asbp_first_person_character)
  (set `/Game/FirstPerson/Blueprints/BP_FirstPersonCharacter.actualInteractObjective` null _asbp_first_person_character))

(event `Interact`
  (`self.DesactivateEvent`)
  (`self.OnEndCondition`)
  (`KismetSystemLibrary.PrintString` "Objective Completed"))

(fn `UserConstructionScript`
  (`parent.UserConstructionScript`))