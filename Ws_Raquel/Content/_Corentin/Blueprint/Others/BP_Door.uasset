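; BP_Door is a door actor that teleports the first-person character to a linked TeleportationPoint.
; A Box overlap casts to BP_FirstPersonCharacter, stores it and, while IsActive is set, moves it to that point's location.
; The teleport uses a hard-coded rotation, then player controller 0's control rotation is set to the point's rotation.
; IsActive turns on at BeginPlay and is never cleared here.
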(event `self.ReceiveBeginPlay`
  (set `self.isActive` true))

(event `self.Box.OnComponentBeginOverlap`
  (params (OverlappedComponent :type "PrimitiveComponent Object Reference") (OtherActor :type "Actor Object Reference") (OtherComp :type "PrimitiveComponent Object Reference") (OtherBodyIndex :type Integer) (bFromSweep :type Boolean) (SweepResult :type "HitResult Structure (by ref)"))
  (bind _asbp_first_person_character (cast `/Game/FirstPerson/Blueprints/BP_FirstPersonCharacter` OtherActor))
  (set `self.Character` _asbp_first_person_character)
  (if (`self.isActive`)
    (`self.K2_TeleportTo` (`self.Character`) (`self.K2_GetActorLocation` (`self.TeleportationPoint`)) (struct :`Yaw` 70.0))
    (`Controller.SetControlRotation` (`GameplayStatics.GetPlayerController` 0) (`self.K2_GetActorRotation` (`self.TeleportationPoint`)))))

(fn `UserConstructionScript`)