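; Kill objective that completes once every mannequin in its Enemies list is dead.
; It deactivates itself and its mannequins on BeginPlay; activation wakes them, binds to each one's death event and prints the objective name.
; The end-condition check recounts dead enemies; when all are dead, it deactivates the objective and calls OnEndCondition.
; Debug prints report activation and check results.
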(event `self.ReceiveBeginPlay`
  (`self.DesactivateEvent`))

(event `self.ActivateEvent`
  (bind _informations_objectivename (break `/Game/_Romain/Utilities/F_Objective` (`self.informations`)))
  (set `self.isActive` true)
  (for _array_element (`self.enemies`)
    (`/Game/_Corentin/Blueprint/BP_Mannequin.ActivateMannequin` _array_element)
    (add `/Game/_Corentin/Blueprint/BP_Mannequin.onDeath` _array_element (`|CreateDelegate` :!event `CheckForEndCondition`)))
  (`KismetSystemLibrary.PrintString` "Event Activate")
  (`KismetSystemLibrary.PrintString` _informations_objectivename true true (struct :`G` 0.66 :`B` 1.0 :`A` 1.0) 5.0))

(event `self.DesactivateEvent`
  (set `self.isActive` false)
  (for _array_element (`self.enemies`)
    (`/Game/_Corentin/Blueprint/BP_Mannequin.DesactivateMannequin` _array_element)))

(event `CheckForEndCondition`
  (for _array_element (`self.enemies`)
    (if (`/Game/_Corentin/Blueprint/BP_Mannequin.isDead` _array_element)
      (`/Engine/EditorBlueprintResources/StandardMacros.IncrementInt` (`self.deadEnemiesIndex`))))
  (if (== (`self.deadEnemiesIndex`) (`KismetArrayLibrary.Array_Length` (`self.enemies`)))
    (set `self.deadEnemiesIndex` 0)
    (`self.DesactivateEvent`)
    (`self.OnEndCondition`)
    (`KismetSystemLibrary.PrintString` "Objective Completed")
    (else
      (set `self.deadEnemiesIndex` 0)
      (`KismetSystemLibrary.PrintString` "Objective Not Completed"))))

(fn `UserConstructionScript`
  (`parent.UserConstructionScript`))