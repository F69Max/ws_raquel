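; BP_Objective_Cutscene is an objective that holds the first-person player in place for a timed cutscene by disabling input.
; On activation it marks itself active, disables input on the character cached at BeginPlay, and waits for a Duration delay.
; It then deactivates itself, restores input, and calls the end condition to signal completion.
; The file only handles the input lock and timing, with no camera or sequence playback.
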(event `self.ReceiveBeginPlay`
  (bind _asbp_first_person_character (cast `/Game/FirstPerson/Blueprints/BP_FirstPersonCharacter` (`GameplayStatics.GetPlayerCharacter` 0)))
  (set `self.character` _asbp_first_person_character))

(event `self.ActivateEvent`
  (set `self.isActive` true)
  (`self.DisableInput` (`self.character`) (`GameplayStatics.GetPlayerController` 0))
  (`KismetSystemLibrary.Delay` (`self.Duration`))
  (`self.DesactivateEvent`)
  (`self.OnEndCondition`))

(event `self.DesactivateEvent`
  (set `self.isActive` false)
  (`self.EnableInput` (`self.character`) (`GameplayStatics.GetPlayerController` 0)))

(fn `UserConstructionScript`
  (`parent.UserConstructionScript`))